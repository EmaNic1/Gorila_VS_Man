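; BP_HealthPickUp is a health pickup actor for the gorilla player character.
; When an actor tagged Player overlaps its trigger component, it casts to BP_Gorila and increases its health by 10.
; It then plays a sound at its location and destroys itself.
; An unconnected leftover chain for updating the gorilla health bar widget never runs.
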(event `self.Triger.OnComponentBeginOverlap`
  (params (OverlappedComponent :type "PrimitiveComponent Object Reference") (OtherActor :type "Actor Object Reference") (OtherComp :type "PrimitiveComponent Object Reference") (OtherBodyIndex :type Integer) (bFromSweep :type Boolean) (SweepResult :type "HitResult Structure (by ref)"))
  (if (`self.ActorHasTag` OtherActor "Player")
    (bind _asbp_gorila (cast `/Game/Blueprint/BP_Gorila` OtherActor))
    (`/Game/Blueprint/BP_Gorila.IncreaseHealth` _asbp_gorila 10.0)
    (`GameplayStatics.PlaySoundAtLocation` "/Engine/VREditor/Sounds/UI/Camera_Shutter.Camera_Shutter" (`self.K2_GetActorLocation`) (struct) 1.0 1.0 0.0 null null null null)
    (`self.K2_DestroyActor`)))

(fn `UserConstructionScript`)