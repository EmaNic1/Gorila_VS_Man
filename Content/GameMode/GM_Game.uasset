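; GM_Game is a game mode Blueprint that scatters health pickups across the level when play begins.
; BeginPlay calls SpawnHealth, which gathers all BP_SapwnHearth actors as candidate spawn points.
; A fixed-count loop picks a random point, spawns BP_HealthPickUp at its location, then removes it from the list and destroys it, so no point is reused.
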(event `self.ReceiveBeginPlay`
  (`self.SpawnHealth`))

(fn `SpawnHealth`
  (locals (`local spawn points` :type "Array of /Game/Blueprint/BP_SapwnHearth Object Reference") (`Local item` :type "/Game/Blueprint/BP_SapwnHearth Object Reference"))
  (bind _outactors (`GameplayStatics.GetAllActorsOfClass` "/Game/Blueprint/BP_SapwnHearth.BP_SapwnHearth_C"))
  (set `local.local spawn points` _outactors)
  (for _ (range 8)
    (set `local.Local item` (`KismetArrayLibrary.Array_Random` (`local.local spawn points`)))
    (`|SpawnActorFromClass` "/Game/Blueprint/BP_HealthPickUp.BP_HealthPickUp_C" (`KismetMathLibrary.MakeTransform` (`self.K2_GetActorLocation` (`local.Local item`))) "AdjustIfPossibleButAlwaysSpawn" "MultiplyWithRoot" null null)
    (`KismetArrayLibrary.Array_RemoveItem` (`local.local spawn points`) (`local.Local item`))
    (`self.K2_DestroyActor` (`local.Local item`))))

(fn `UserConstructionScript`)